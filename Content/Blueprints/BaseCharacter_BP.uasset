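; BaseCharacter_BP is a character base with health, damage handling and a scored death.
; Construction sets Health to HealthMax, and AnyDamage subtracts damage, then re-evaluates Health minus Damage for the death check, so death triggers one equal hit early.
; CharacterDeath spawns the death effect, adds KillScore through the MyGame game mode and destroys the actor.
; If the game mode cast fails, the actor is not destroyed.
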(event EventAnyDamage
  (params (Damage :type Float%20%28single-precision%29) (DamageType :type Damage%20Type%20Object%20Reference) (InstigatedBy :type Controller%20Object%20Reference) (DamageCauser :type Actor%20Object%20Reference))
  (Variables|Default|SetHealth (- (Variables|Default|GetHealth) Damage))
  (if (not (> (- (Variables|Default|GetHealth) Damage) 0.0))
    (CallFunction|CharacterDeath)))

(fn ConstructionScript
  (Variables|Default|SetHealth (Variables|Default|GetHealthMax)))

(fn CharacterDeath
  (Effects|SpawnEmitteratLocation (Variables|Default|GetDeathEffect) (Transformation|GetActorLocation))
  (bind _asmygame_c (Utilities|Casting|CastToMyGame (Game|GetGameMode)))
  (Default|AddScore _asmygame_c (Variables|Default|GetKillScore))
  (Actor|DestroyActor))