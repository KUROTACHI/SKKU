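; MyEnemy is an enemy that walks back and forth along the Y axis, damaging and knocking back what it runs into.
; Tick feeds MoveValue into movement input, and Hit flips its sign from the hit normal's Y to send the enemy away from the obstacle.
; Hit applies VelocityDamage to anything except another MyEnemy, while VelocityTarget launches any Character hit by setting Falling mode and overwriting its velocity.
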(event EventHit
  (params (MyComp :type Primitive%20Component%20Object%20Reference) (Other :type Actor%20Object%20Reference) (OtherComp :type Primitive%20Component%20Object%20Reference) (bSelfMoved :type Boolean) (HitLocation :type Vector :default "0, 0, 0") (HitNormal :type Vector :default "0, 0, 0") (NormalImpulse :type Vector :default "0, 0, 0") (Hit :type Hit%20Result%20Structure%20%28by%20ref%29))
  (bind _y (Math|Vector|BreakVector HitNormal))
  (Utilities|Casting|CastToMyEnemy Other
    (:then
      _)
    (:CastFailed
      (Game|Damage|ApplyDamage Other (Variables|Default|GetVelocityDamage) 0 0)))
  (CallFunction|VelocityTarget Other _y)
  (Math|Float|CompareFloat _y 0.0
    (:>
      (CallFunction|ToggleMoveDirection false))
    (:<
      (CallFunction|ToggleMoveDirection true))))

(event EventTick
  (params (DeltaSeconds :type Float%20%28single-precision%29))
  (Pawn|Input|AddMovementInput "0,-1.000000, 0" (Variables|Default|GetMoveValue)))

(fn ConstructionScript)

(fn ToggleMoveDirection
  (params (Toggle :type Boolean))
  (if Toggle
    (Variables|Default|SetMoveValue 1.0)
    (else
      (Variables|Default|SetMoveValue -1.0))))

(fn VelocityTarget
  (params (TargetActor :type Object%20Object%20Reference) (Velocity :type Float%20%28single-precision%29))
  (bind _ascharacter (Utilities|Casting|CastToCharacter TargetActor))
  (bind _ascharactermovementcomponent (Utilities|Casting|CastToCharacterMovementComponent (Pawn|GetMovementComponent _ascharacter)))
  (Pawn|Components|CharacterMovement|SetMovementMode _ascharactermovementcomponent "MOVE_Falling" 0)
  (Variables|/Script/Engine.MovementComponent|SetVelocity (Pawn|GetMovementComponent _ascharacter) (Math|Vector|MakeVector 0.0 (* Velocity -5e+02) 5e+02)))